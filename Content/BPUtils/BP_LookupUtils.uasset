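; Blueprint utility that maps Veggle gameplay tags to display assets for vegetables and flavours.
; GetFlavorIconByTag switches on a flavour tag, including a wildcard flavour, and returns the matching icon texture.
; GetVeggieMeshFromTag switches on a vegetable tag and returns its mesh.
; Both are hard-coded tag switches with no fallback asset for unmatched tags.
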(fn `GetFlavorIconByTag`
  (params (InTag :type "GameplayTag Structure"))
  (returns (OutIcon :type "Texture2D Object Reference"))
  (`|SwitchGameplayTag` InTag
    (:`Veggle.Flavour.Butter`
      (return "/Game/Images/T_Butter.T_Butter"))
    (:`Veggle.Flavour.Heat`
      (return "/Game/Images/T_Heat.T_Heat"))
    (:`Veggle.Flavour.Pepper`
      (return "/Game/Images/T_Pepper.T_Pepper"))
    (:`Veggle.Flavour.Salt`
      (return "/Game/Images/T_Salt.T_Salt"))
    (:`Veggle.Flavour.WildcardFlavour`
      (return "/Game/Images/T_Wildcard.T_Wildcard"))))

(fn `GetVeggieMeshFromTag`
  (params (VeggieTag :type "GameplayTag Structure"))
  (returns (Mesh :type "StaticMesh Object Reference"))
  (`|SwitchGameplayTag` VeggieTag
    (:`Veggle.Vegetable.Carrot`
      (return "/Game/Mesh/Veggies/Carrot/SM_Carrot.SM_Carrot"))
    (:`Veggle.Vegetable.Corn`
      (return "/Game/Mesh/Veggies/Corn/S_Corn.S_Corn"))
    (:`Veggle.Vegetable.Onion`
      (return "/Game/Mesh/Veggies/Onion/SM_Onion.SM_Onion"))
    (:`Veggle.Vegetable.Potato`
      (return "/Game/Mesh/Veggies/Potato/SM_Potato.SM_Potato"))
    (:`Veggle.Vegetable.Tomato`
      (return "/Game/Mesh/Veggies/Tomato/SM_Tomato.SM_Tomato"))))