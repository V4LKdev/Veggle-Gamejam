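; BP_VeggleWalker is a hopping vegetable character with randomized scale and yaw, and voice sounds during play and after game end.
; Hops apply a sideways-and-up capsule impulse in a random direction, forced one way after game end so veggies exit offscreen.
; Timelines squash and stretch mesh Z using per-veggie-type tuning.
; A DoOnce-gated hit triggers landing, which schedules the next hop, with Tick forcing one after a timeout.
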(event `self.ReceiveBeginPlay`
  (bind _veggiemesh (`self.VeggieMesh`))
  (bind _output_get (set `self.MeshScale` (`KismetMathLibrary.VLerp` (0.8 0.8 0.8) (1.2 1.2 1.2) (`KismetMathLibrary.RandomFloat`))))
  (`SceneComponent.SetRelativeScale3D` _veggiemesh _output_get)
  (`SceneComponent.K2_SetRelativeRotation` _veggiemesh (`KismetMathLibrary.MakeRotator` 0.0 0.0 (`KismetMathLibrary.RandomFloatInRange` -30.0 30.0)) false false))

(event `self.BP_OnVeggieClicked`
  (params (TouchedActor :type "Actor Object Reference") (ButtonPressed :type "Key Structure")))

(event `self.ReceiveTick`
  (params (DeltaSeconds :type "Float (single-precision)"))
  (bind _output_get (set `self.TimeSinceLastHop` (+ DeltaSeconds (`self.TimeSinceLastHop`))))
  (if (> _output_get 5.0)
    (`self.Hop`)))

(event `ResetLanding`
  (goto _label :!via `Reset`))

(event `self.BP_OnVeggieHit`
  (params (HitComponent :type "PrimitiveComponent Object Reference") (OtherActor :type "Actor Object Reference") (OtherComp :type "PrimitiveComponent Object Reference") (NormalImpulse :type "Vector Structure") (Hit :type "HitResult Structure (by ref)"))
  (`/Engine/EditorBlueprintResources/StandardMacros.DoOnce` false :!label _label
    (:`Completed`
      (`TimelineComponent.SetPlayRate` (`self.T_Landing`) (`VeggleWalkingVeggieData.LandingSpeedMultiplier` (`self.GetVeggieType`)))
      (`GameplayStatics.PlaySound2D` "/Game/Sounds/VeggieBounce/MS_Bounce.MS_Bounce" 1.0 1.0 0.0 null null)
      (bind (_direction _alpha) (`Timeline|T_Landing` :!via `PlayFromStart`)
        (:`Update`
          (`self.LerpMeshZ` (`VeggleWalkingVeggieData.LandingZScale` (`self.GetVeggieType`)) _alpha))
        (:`Finished`
          (`KismetSystemLibrary.K2_SetTimerDelegate` (`|CreateDelegate` :!event `Hop`) (`self.GetRandomTimeToNextHop`)))))))

(event `Hop`
  (`TimelineComponent.SetPlayRate` (`self.T_Hop`) (`VeggleWalkingVeggieData.HopSpeedMultiplier` (`self.GetVeggieType`)))
  (`|ExecutionSequence`
    (:`then_0`
      (set `self.TimeSinceLastHop` 0.0)
      (bind (_direction _alpha) (`Timeline|T_Hop` :!via `PlayFromStart`)
        (:`Update`
          (`self.LerpMeshZ` (`VeggleWalkingVeggieData.HopZScale` (`self.GetVeggieType`)) _alpha))
        (:`Hop`
          (`self.AddHopImpulse`)
          (`self.ResetLanding`))))
    (:`then_1`
      (if (and (`KismetMathLibrary.RandomBoolWithWeight` 0.2) (not (`self.bGameEnded`)))
        (`GameplayStatics.PlaySound2D` "/Game/Sounds/Veggies/MS_Veggies.MS_Veggies" 1.0 1.0 0.0 null null)))))

(event `self.BP_OnGameEnded`
  (`KismetSystemLibrary.Delay` (`KismetMathLibrary.RandomFloatInRange` 1.0 15.0))
  (if (`KismetMathLibrary.RandomBoolWithWeight` 0.8)
    (`GameplayStatics.PlaySound2D` "/Game/Sounds/Veggies/MS_Bye.MS_Bye" 1.0 1.0 0.0 null null)))

(fn `AddHopImpulse`
  (bind _returnvalue (`self.GetVeggieType`))
  (bind _hopsidestrength (`VeggleWalkingVeggieData.HopSideStrength` _returnvalue))
  (`PrimitiveComponent.AddImpulse` (`self.CapsuleCollision`) (`KismetMathLibrary.MakeVector` 0.0 (`KismetMathLibrary.SelectFloat` (* _hopsidestrength -1.0) _hopsidestrength (`self.GetRandomHopLeft`)) (`KismetMathLibrary.Abs` (`VeggleWalkingVeggieData.HopUpStrength` _returnvalue))) "None" true))

(fn `UserConstructionScript`)