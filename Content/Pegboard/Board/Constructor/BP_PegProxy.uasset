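; BP_PegProxy is a placeholder peg actor for constructing pegboards.
; SetupProxy stores a peg type and shows its tag name on a text component.
; GetBakeData packages the static mesh's world transform and peg type as peg instance data for baking.
; BeginPlay prints a warning that proxy pegs remain in the scene.
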(event `self.ReceiveBeginPlay`
  (`KismetSystemLibrary.PrintString` "There is one or more Proxy Peg in the Scene!" true true (struct :`R` 1.0 :`G` 0.904897 :`A` 1.0) 2.0 "ProxyPeg"))

(fn `GetBakeData`
  (returns (OutData :type "VegglePegInstanceData Structure"))
  (return (make `VegglePegInstanceData` (`SceneComponent.K2_GetComponentToWorld` (`self.StaticMesh`)) (`self.PegType`))))

(fn `SetupProxy`
  (params (PegType :type "VegglePegData Object Reference"))
  (bind _output_get (set `self.PegType` PegType))
  (`TextRenderComponent.K2_SetText` (`self.TypeText`) (`KismetTextLibrary.Conv_NameToText` (`BlueprintGameplayTagLibrary.GetTagName` (`VegglePegData.PegTypeTag` _output_get)))))

(fn `UserConstructionScript`)