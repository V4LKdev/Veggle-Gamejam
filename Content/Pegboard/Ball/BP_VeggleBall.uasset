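; Pegboard ball actor that adds a constant downward force to its mesh while physics is simulated.
; Hitting an active peg plays a MetaSound fed the running hit count, so the sound can vary along a streak.
; For pegs with a valid type tag, it shows a score widget at the ball's location if its ability system's count of that tag is at most one.
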(event `self.ReceiveTick`
  (params (DeltaSeconds :type "Float (single-precision)"))
  (bind _ballmesh (`self.BallMesh`))
  (if (`SceneComponent.IsSimulatingPhysics` _ballmesh "None")
    (`PrimitiveComponent.AddForce` _ballmesh (0.0 0.0 -200.0) "None" false)))

(event `self.BP_OnBallHit`
  (params (HitPegData :type "VegglePegData Object Reference") (bHitActivePeg :type Boolean))
  (bind _pegtypetag (`VegglePegData.PegTypeTag` HitPegData))
  (if bHitActivePeg
    (bind _returnvalue (`GameplayStatics.SpawnSound2D` "/Game/Sounds/PegHit/MS_PegHit.MS_PegHit" 1.0 1.0 0.0 null))
    (`AudioParameterControllerInterface.SetIntParameter` _returnvalue "Hits" (`self.Hits`))
    (`/Engine/EditorBlueprintResources/StandardMacros.IncrementInt` (`self.Hits`)
      (:`  `
        (if (`BlueprintGameplayTagLibrary.IsGameplayTagValid` _pegtypetag)
          (if (<= (`AbilitySystemComponent.GetGameplayTagCount` (`self.AbilitySystemComponent`) _pegtypetag) 1)
            (bind _returnvalue_2 (`|CreateWidget` "/Game/Widget/Scoring/WBP_PegScore.WBP_PegScore_C" null 1.0 (`self.K2_GetActorLocation`)))
            (`UserWidget.AddToViewport` _returnvalue_2 0)))))))

(fn `UserConstructionScript`)