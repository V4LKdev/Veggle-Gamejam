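; BP_MusicActor plays background music, kitchen ambience and a no-hit sound effect for the Veggle pegboard game.
; On BeginPlay it creates the two looping-bed audio components and binds to game state and Veggle event subsystem events.
; Both tracks fade in when the pregame countdown starts and fade out when postgame starts.
; A veggie evaluated as a no-hit triggers a one-shot 2D sound.
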(event `self.ReceiveBeginPlay`
  (bind _returnvalue (`VeggleGameUtils.GetVeggleGameState`))
  (add `VeggleGameState.OnPregameCountdownStarted` _returnvalue (delegate `FadeInMusic`))
  (add `VeggleGameState.OnPostgameStarted` _returnvalue (delegate `FadeOutMusic`))
  (`|ExecutionSequence`
    (:`then_0`
      (add `VeggleEventSubsystem.OnVeggieEvaluated` (`VeggleGameUtils.GetVeggleEventSubsystem`) (`|CreateDelegate` :!event `OnVeggieEval`)))
    (:`then_1`
      (bind _returnvalue_2 (`GameplayStatics.CreateSound2D` "/Game/Sounds/KitchenAmbience_Cue.KitchenAmbience_Cue" 1.0 1.0 0.0 null))
      (set `self.AmbienceSound` _returnvalue_2)
      (bind _returnvalue_3 (`GameplayStatics.CreateSound2D` "/Game/Sounds/Lobo_Loco_-_Lights_Trip__ID_2364__Cue.Lobo_Loco_-_Lights_Trip__ID_2364__Cue" 1.0 1.0 0.0 null))
      (set `self.BGMusic` _returnvalue_3))))

(event `FadeInMusic`
  (`AudioComponent.FadeIn` (`self.AmbienceSound`) 3.0 1.0 0.0 "Linear")
  (`AudioComponent.FadeIn` (`self.BGMusic`) 3.0 1.0 0.0 "Linear"))

(event `FadeOutMusic`
  (`AudioComponent.FadeOut` (`self.AmbienceSound`) 3.0 0.0 "Linear")
  (`AudioComponent.FadeOut` (`self.BGMusic`) 3.0 0.0 "Linear"))

(event `OnVeggieEval`
  (params (Payload :type "VeggieEvaluatedPayload Structure (by ref)"))
  (if (`.bWasNoHit` (break `VeggieEvaluatedPayload` Payload))
    (`GameplayStatics.PlaySound2D` "/Game/Sounds/NoHit.NoHit" 0.7 1.0 0.3 null null)))

(fn `UserConstructionScript`)