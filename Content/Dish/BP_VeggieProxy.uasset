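; BP_VeggieProxy is a physics-simulated stand-in for a vegetable, with its mesh chosen from a Tag.
; On BeginPlay, a valid mesh from GetVeggieMeshFromTag is applied and physics is switched on.
; It then optionally self-destructs on a short timer and optionally tumbles with a random angular velocity change.
; The tumble uses one random alpha for the vector lerp, so spin always follows the same diagonal axis.
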(event `self.ReceiveBeginPlay`
  (bind _staticmeshcomponent (`self.StaticMeshComponent`))
  (bind _mesh (`/Game/BPUtils/BP_LookupUtils.GetVeggieMeshFromTag` (`self.Tag`)))
  (`/Engine/EditorBlueprintResources/StandardMacros.IsValid` _mesh
    (:`Is Valid`
      (`StaticMeshComponent.SetStaticMesh` _staticmeshcomponent _mesh)
      (`PrimitiveComponent.SetSimulatePhysics` _staticmeshcomponent true)
      (`|ExecutionSequence`
        (:`then_0`
          (if (`self.bAutoDestroy`)
            (`KismetSystemLibrary.K2_SetTimerDelegate` (delegate `Destroy`) 5.0)))
        (:`then_1`
          (if (`self.bTumble`)
            (`PrimitiveComponent.AddAngularImpulseInDegrees` (`self.StaticMeshComponent`) (`KismetMathLibrary.VLerp` (-100.0 -100.0 -100.0) (100.0 100.0 100.0) (`KismetMathLibrary.RandomFloat`)) "None" true)))))))

(event `Destroy`
  (`self.K2_DestroyActor`))

(fn `UserConstructionScript`)