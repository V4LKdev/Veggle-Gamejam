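; BP_VeggleDish is a dish actor that slides into place on spawn and slides away when served.
; Timelines lerp it along a Y offset from its starting location, with a plate-drag sound each way.
; SpawnVeggieProxy drops tagged BP_VeggieProxy actors above the dish at a random Y offset and tracks them.
; ServeDish waits briefly, slides out, fires OnDishServed, then after a delay destroys the proxies and itself.
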(event `self.ReceiveBeginPlay`
  (bind (_dishloc_x _dishloc_y _dishloc_z) (`KismetMathLibrary.BreakVector` (`self.DishLoc`)))
  (bind _dishloc (`self.DishLoc`))
  (set `self.DishLoc` (`self.K2_GetActorLocation`))
  (`GameplayStatics.PlaySound2D` "/Game/Sounds/PlateDrag/MS_PlateDrag.MS_PlateDrag" 1.0 1.0 0.0 null null)
  (bind (_direction _alpha) (`Timeline|TL_Spawn` :!via `PlayFromStart`)
    (:`Update`
      (`self.K2_SetActorLocation` (`KismetMathLibrary.VLerp` (`KismetMathLibrary.MakeVector` _dishloc_x (+ _dishloc_y 1000.0) _dishloc_z) _dishloc _alpha)))
    (:`Finished`
      (`self.K2_SetActorLocation` _dishloc))))

(event `self.ServeDish`
  (bind (_dishloc_x _dishloc_y _dishloc_z) (`KismetMathLibrary.BreakVector` (`self.DishLoc`)))
  (`KismetSystemLibrary.Delay` 1.0)
  (`GameplayStatics.PlaySound2D` "/Game/Sounds/PlateDrag/MS_PlateDrag.MS_PlateDrag" 1.0 1.0 0.0 null null)
  (bind (_direction _alpha) (`Timeline|TL_Despawn` :!via `PlayFromStart`)
    (:`Update`
      (`self.K2_SetActorLocation` (`KismetMathLibrary.VLerp` (`self.DishLoc`) (`KismetMathLibrary.MakeVector` _dishloc_x (+ _dishloc_y 1000.0) _dishloc_z) _alpha)))
    (:`Finished`
      (`self.OnDishServed`)
      (`KismetSystemLibrary.Delay` 2.0)
      (for _array_element (`self.ProxyVeggies`)
        (`self.K2_DestroyActor` _array_element))
      (`self.K2_DestroyActor`))))

(event `self.SpawnVeggieProxy`
  (params (InVeggieTag :type "GameplayTag Structure (by ref)") (bWasCorrect :type Boolean))
  (bind (_dishloc_x _dishloc_y _dishloc_z) (`KismetMathLibrary.BreakVector` (`self.DishLoc`)))
  (bind _returnvalue (`|SpawnActorFromClass` "/Game/Dish/BP_VeggieProxy.BP_VeggieProxy_C" (`KismetMathLibrary.MakeTransform` (`KismetMathLibrary.MakeVector` _dishloc_x (+ _dishloc_y (`KismetMathLibrary.RandomFloatInRange` -50.0 50.0)) (+ _dishloc_z 500.0))) "Undefined" "MultiplyWithRoot" null InVeggieTag false false null))
  (`KismetArrayLibrary.Array_Add` (`self.ProxyVeggies`) _returnvalue))

(fn `UserConstructionScript`)