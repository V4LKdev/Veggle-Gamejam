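; BP_VeggieDropper is a main menu actor that continuously spawns decorative vegetables.
; A looping half-second timer started on BeginPlay spawns BP_VeggieProxy actors at random points along a line between two offsets from its location.
; Each proxy gets a random yaw, scale and gameplay tag choosing one of five vegetable types, and is set to tumble and auto-destroy.
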(event `self.ReceiveBeginPlay`
  (bind _returnvalue (`KismetSystemLibrary.K2_SetTimerDelegate` (delegate `SpawnVeggie`) 0.5 true))
  (set `self.SpawnHandle` _returnvalue))

(event `SpawnVeggie`
  (bind _returnvalue (`KismetMathLibrary.RandomFloat`))
  (`|SpawnActorFromClass` "/Game/Dish/BP_VeggieProxy.BP_VeggieProxy_C" (`KismetMathLibrary.MakeTransform` (+ (`self.K2_GetActorLocation`) (`KismetMathLibrary.VLerp` (`self.SpawnA`) (`self.SpawnB`) _returnvalue)) (`KismetMathLibrary.MakeRotator` 0.0 0.0 (`KismetMathLibrary.RandomFloatInRange` -45.0 45.0)) (`KismetMathLibrary.VLerp` (0.8 0.8 0.8) (1.5 1.5 1.5) _returnvalue)) "Undefined" "MultiplyWithRoot" null (`KismetArrayLibrary.Array_Random` (`|MakeArray` (struct :`TagName` "Veggle.Vegetable.Carrot") (struct :`TagName` "Veggle.Vegetable.Corn") (struct :`TagName` "Veggle.Vegetable.Onion") (struct :`TagName` "Veggle.Vegetable.Potato") (struct :`TagName` "Veggle.Vegetable.Tomato") :!type "GameplayTag Structure")) true true null))

(fn `UserConstructionScript`)